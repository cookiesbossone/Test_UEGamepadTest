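; BP_GamepadDetectActor is a debug actor that reports registered input devices when its OnGamepadConnection event fires.
; It prints the device count in red, then loops over GetRegisteredDevices to print each DeviceName.
; It splits each name on backslashes and parses the third segment to extract VID and PID, printing both with screen output disabled.
; BeginPlay, overlap, Tick and the construction script are empty.
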(event `self.ReceiveBeginPlay`)

(event `self.ReceiveActorBeginOverlap`
  (params (OtherActor :type "Actor Object Reference")))

(event `self.ReceiveTick`
  (params (DeltaSeconds :type "Float (single-precision)")))

(event `self.OnGamepadConnection`
  (bind _returnvalue (`KismetArrayLibrary.Array_Length` (`RawInputFunctionLibrary.GetRegisteredDevices`)))
  ;[1 1 1] 打印当前连接的Device数量
  (`KismetSystemLibrary.PrintString` (`KismetStringLibrary.Concat_StrStr` "Now Gamepad Num : " (`KismetStringLibrary.Conv_IntToString` _returnvalue)) true true (struct :`R` 1.0 :`G` 0.110466 :`A` 1.0))
  (if (not (== _returnvalue 0))
    (for _array_element (`RawInputFunctionLibrary.GetRegisteredDevices`)
      (bind (_handle _vendorid _productid _devicename) (break `RegisteredDeviceInfo` _array_element))
      (`KismetSystemLibrary.PrintString` (`KismetStringLibrary.Concat_StrStr` "DeviceName = " _devicename))
      (for (_array_element_2 _array_index) (`KismetStringLibrary.ParseIntoArray` _devicename "\\")
        (if (== _array_index 2)
          (bind _returnvalue_2 (`KismetStringLibrary.ParseIntoArray` (`KismetStringLibrary.Replace` _array_element_2 "&" "_") "_"))
          (`KismetSystemLibrary.PrintString` (`KismetStringLibrary.Concat_StrStr` "VID = " (`|GetArrayItem` _returnvalue_2 1)) false)
          (`KismetSystemLibrary.PrintString` (`KismetStringLibrary.Concat_StrStr` "PID = " (`|GetArrayItem` _returnvalue_2 3)) false))))))

(fn `UserConstructionScript`)